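; Firebolt gameplay ability that casts a projectile toward the location under the mouse.
; A target-data task stores the hit location, and the ability commits and passes that location to the avatar as a motion-warp target.
; It plays the cast montage, spawns the projectile on the montage's Firebolt gameplay event, and ends when the montage completes.
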(event `self.K2_ActivateAbility`
  (bind (_asynctaskproxy _datahandle) (`TargetDataUnderMouse.CreateTargetDataUnderMouse`)
    (:`then`
      (`self.K2_CommitAbility`)
      (message `CombatInterface.SetWarpTargetLocation` (`self.GetAvatarActorFromActorInfo`) (`self.Projectile Target Location`))
      (`AbilityTask_PlayMontageAndWait.CreatePlayMontageAndWaitProxy` "None" "/Game/Assets/Characters/Aura/Animations/Abilities/AM_Cast_Firebolt.AM_Cast_Firebolt"
        (:`then`
          (`AbilityTask_WaitGameplayEvent.WaitGameplayEvent` (struct :`TagName` "Event.Montage.Firebolt") null
            (:`EventReceived`
              (`self.SpawnProjectile` (`self.Projectile Target Location`)))))
        (:`OnCompleted`
          (`self.K2_EndAbility`))))
    (:`ValidData`
      (bind (_returnvalue_bblockinghit _returnvalue_binitialoverlap _returnvalue_time _returnvalue_distance _returnvalue_location) (`GameplayStatics.BreakHitResult` (`AbilitySystemBlueprintLibrary.GetHitResultFromTargetData` _datahandle)))
      (set `self.Projectile Target Location` _returnvalue_location))))