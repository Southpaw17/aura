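; Melee attack gameplay ability that warps the avatar toward its combat target and plays a random attack montage from the avatar's list.
; A gameplay event matching the montage's tag triggers a small sphere query at that tag's combat socket, damaging every live player found except the attacker.
; Avatar data comes through interface messages, and the ability ends when the montage completes, is interrupted or is cancelled.
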(event `self.K2_ActivateAbility`
  (bind _returnvalue (`self.GetAvatarActorFromActorInfo`))
  (bind _returnvalue_2 (`self.GetAvatarActorFromActorInfo`))
  (bind _returnvalue_3 (`self.K2_CommitAbility`))
  (if _returnvalue_3
    (bind _returnvalue_4 (message `InteractableInterface.GetCombatTarget` _returnvalue))
    (message `CombatInterface.SetWarpTargetLocation` _returnvalue (`Actor.K2_GetActorLocation` _returnvalue_4))
    (bind _output_get (set `self.Tagged Montage` (`self.GetRandomTaggedMontage`)))
    (`AbilityTask_PlayMontageAndWait.CreatePlayMontageAndWaitProxy` "None" (break `TaggedMontage` _output_get)
      (:`then`
        (`AbilityTask_WaitGameplayEvent.WaitGameplayEvent` (`.MontageTag` (break `TaggedMontage` _output_get)) null true
          (:`EventReceived`
            (bind _returnvalue_5 (message `CombatInterface.GetCombatSocketLocation` _returnvalue_2 (`.MontageTag` (break `TaggedMontage` _output_get))))
            (bind _outoverlappingactors (`AuraAbilitySystemLibrary.GetLivePlayersWithinRadius` _returnvalue_2 (`|MakeArray` _returnvalue_2) 45.0 _returnvalue_5))
            (for _array_element _outoverlappingactors
              (`self.CauseDamage` _array_element)))))
      (:`OnCompleted`
        (`self.K2_EndAbility` :!label _label))
      (:`OnInterrupted`
        (goto _label))
      (:`OnCancelled`
        (goto _label)))))

(fn `GetRandomTaggedMontage`
  (returns (`Tagged Montage` :type "TaggedMontage Structure"))
  (bind _returnvalue (message `CombatInterface.GetAttackMontages` (`self.GetAvatarActorFromActorInfo`)))
  (return (`|GetArrayItem` _returnvalue (`KismetMathLibrary.RandomIntegerInRange` 0 (- (`KismetArrayLibrary.Array_Length` _returnvalue) 1)))))